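; Player pawn for a size-changing level game, where BP_PickUp overlaps shrink it and BP_Meta overlaps win.
; Grow, shrink, death and animations-done events drive sounds, input and a change-screen widget.
; Tick feeds grow-timer progress into a material blend and triggers the looping move audio from left-mouse input, with its Size parameter following pawn scale.
; Winning advances the game instance's level, returning to the menu after level seven.
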(event EventEWinEvent
  (bind _aslevels (Utilities|Casting|CastToLevels (Game|GetGameInstance)))
  (if (< (+ (Variables|/Game/Menu/Levels.Levels_C|GetCurrentLevel _aslevels) 1) 8)
    (bind _output_get (Variables|/Game/Menu/Levels.Levels_C|SetCurrentLevel _aslevels (+ (Variables|/Game/Menu/Levels.Levels_C|GetCurrentLevel _aslevels) 1)))
    (Game|OpenLevel(byName) (Utilities|String|StringToName (Utilities|String|BuildString(Integer) (Utilities|String|ToString(Name) (Variables|Default|GetLvl_)) "" _output_get)))
    (else
      (Variables|/Game/Menu/Levels.Levels_C|SetCurrentLevel _aslevels 1)
      (Game|OpenLevel(byName) "Menu"))))

(event EventTick
  (params (DeltaSeconds :type Float%20%28single-precision%29))
  (bind _charactermesh (Variables|Default|GetCharacterMesh))
  (Rendering|Material|SetScalarParameterValueonMaterials _charactermesh "Blending" (Class|KismetSystemLibrary|GetTimerElapsedTimeHandle (Variables|/Script/Project_E.SizeManagerComponent|GetGrowTimeHandle (Variables|Default|GetSizeComponent))))
  (Rendering|Material|SetMaterial _charactermesh 0 "/Game/Materials/ERedBlend.ERedBlend")
  (if (Audio|Components|Audio|IsPlaying (Variables|Default|GetMove))
    (if (Game|Player|IsInputKeyDown (Game|GetPlayerController 0) "LeftMouseButton")
      (if (not (Variables|Default|GetisSoundMovePlaying))
        (Variables|Default|SetisSoundMovePlaying true)
        (Class|AudioParameterControllerInterface|SetTriggerParameter (Variables|Default|GetMove) "Start"))
      (elif (Variables|Default|GetisSoundMovePlaying)
        (Variables|Default|SetisSoundMovePlaying false)
        (Class|AudioParameterControllerInterface|SetTriggerParameter (Variables|Default|GetMove) "End")))))

(event EventEDiedEvent
  (Input|DisableInput (Game|GetPlayerController 0))
  (Audio|Components|Audio|Stop (Variables|Default|GetMove))
  (Audio|PlaySound2D "/Game/Audio/MetaSounds/MS_Die.MS_Die" 1.0 1.0 0.0 0 0)
  (bind _returnvalue (UserInterface|CreateWidget "/Game/Menu/BP_ChangeScreen.BP_ChangeScreen_C"))
  (UserInterface|Viewport|AddtoViewport _returnvalue 0))

(event Collision|EventActorBeginOverlap
  (params (OtherActor :type Actor%20Object%20Reference))
  (bind _asbp_pick_up (Utilities|Casting|CastToBP_PickUp OtherActor)
    (:then
      (Actor|DestroyActor _asbp_pick_up)
      (Class|SizeManagerComponent|ShrinkPawn (Actor|GetComponentbyClass self "/Script/Project_E.SizeManagerComponent")))
    (:CastFailed
      (Utilities|Casting|CastToBP_Meta OtherActor)
      (Class|EPawn|Win self))))

(event EventEAnimationsDoneEvent
  (Utilities|IsValid (stale EventEDiedEvent _returnvalue)
    (:Is%20Valid
      (Default|Remove (stale EventEDiedEvent _returnvalue)))
    (:Is%20Not%20Valid
      _))
  (Input|EnableInput (Game|GetPlayerController 0))
  (Audio|Components|Audio|Play (Variables|Default|GetMove) 0.0)
  (Variables|Default|SetisSoundMovePlaying false)
  (Audio|Parameter|SetFloatParameter (Variables|Default|GetMove) "Size" 0.0 :!class /Script/AudioExtensions.AudioParameterControllerInterface))

(event EventBeginPlay
  (UserInterface|Viewport|AddtoViewport (Variables|Default|GetTimerWidgetRef self) 0))

(event EventEGrowEvent
  (Audio|PlaySound2D "/Game/Audio/MetaSounds/MS_Grow.MS_Grow" 1.0 1.0 0.0 0 0)
  (Audio|Parameter|SetFloatParameter (Variables|Default|GetMove) "Size" (/ (Math|Float|Power (- 1.0 (.x (Variables|/Script/Project_E.SizeManagerComponent|GetAnimationEndScale (Variables|Default|GetSizeComponent)))) 3.0) 3.0) :!class /Script/AudioExtensions.AudioParameterControllerInterface))

(event EventEShrinkEvent
  (Audio|PlaySound2D "/Game/Audio/MetaSounds/MS_Shrink.MS_Shrink" 1.0 1.0 0.0 0 0)
  (Audio|Parameter|SetFloatParameter (Variables|Default|GetMove) "Size" (/ (Math|Float|Power (- 1.0 (.x (Variables|/Script/Project_E.SizeManagerComponent|GetAnimationEndScale (Variables|Default|GetSizeComponent)))) 3.0) 3.0) :!class /Script/AudioExtensions.AudioParameterControllerInterface))

(fn ConstructionScript)